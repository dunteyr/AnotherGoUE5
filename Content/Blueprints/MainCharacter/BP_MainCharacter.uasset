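; Player character Blueprint with Enhanced Input movement, look, sprint, jump, slow-motion toggle and ragdoll.
; Walking scales movement input by the walk-to-sprint speed ratio, with max speed fixed at sprint speed.
; Tick tracks horizontal and vertical speed, and jumps at walking speed or slower get a short delay.
; Ragdoll simulates physics from the hips down the bone chain with a loose physical animation profile, with no recovery.
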(event Input|EnhancedActionEvents|EnhancedInputActionIA_MoveForwardCC
  (params (ActionValue :type Float%20%28double-precision%29) (ElapsedSeconds :type Float%20%28double-precision%29) (TriggeredSeconds :type Float%20%28double-precision%29) (InputAction :type Input%20Action%20Object%20Reference :default "/Game/Blueprints/MainCharacter/Input/IA_MoveForwardCC.IA_MoveForwardCC"))
  ;[1 1 1] Movement
  (:Triggered
    (Pawn|Input|AddMovementInput (Math|Vector|GetForwardVector (Math|Rotator|MakeRotator 0.0 0.0 (.Yaw (Math|Rotator|BreakRotator (Pawn|GetControlRotation :!class /Script/Engine.Pawn))))) (* ActionValue (Variables|Default|GetWalkMod)) false)))

(event Input|EnhancedActionEvents|EnhancedInputActionIA_LookUpCC
  (params (ActionValue :type Float%20%28double-precision%29) (ElapsedSeconds :type Float%20%28double-precision%29) (TriggeredSeconds :type Float%20%28double-precision%29) (InputAction :type Input%20Action%20Object%20Reference :default "/Game/Blueprints/MainCharacter/Input/IA_LookUpCC.IA_LookUpCC"))
  ;[1 1 1] Movement
  (:Triggered
    (Pawn|Input|AddControllerPitchInput (* ActionValue (Math|Float|MakeLiteralFloat -1.0)))))

(event Input|EnhancedActionEvents|EnhancedInputActionIA_MoveRightCC
  (params (ActionValue :type Float%20%28double-precision%29) (ElapsedSeconds :type Float%20%28double-precision%29) (TriggeredSeconds :type Float%20%28double-precision%29) (InputAction :type Input%20Action%20Object%20Reference :default "/Game/Blueprints/MainCharacter/Input/IA_MoveRightCC.IA_MoveRightCC"))
  ;[1 1 1] Movement
  (:Triggered
    (Pawn|Input|AddMovementInput (Math|Vector|GetRightVector (Math|Rotator|MakeRotator 0.0 0.0 (.Yaw (Math|Rotator|BreakRotator (Pawn|GetControlRotation :!class /Script/Engine.Pawn))))) (* ActionValue (Variables|Default|GetWalkMod)) false)))

(event Input|EnhancedActionEvents|EnhancedInputActionIA_TurnCC
  (params (ActionValue :type Float%20%28double-precision%29) (ElapsedSeconds :type Float%20%28double-precision%29) (TriggeredSeconds :type Float%20%28double-precision%29) (InputAction :type Input%20Action%20Object%20Reference :default "/Game/Blueprints/MainCharacter/Input/IA_TurnCC.IA_TurnCC"))
  ;[1 1 1] Movement
  (:Triggered
    (Pawn|Input|AddControllerYawInput ActionValue)))

(event Input|EnhancedActionEvents|EnhancedInputActionIA_SprintCC
  (params (ActionValue :type Boolean) (ElapsedSeconds :type Float%20%28double-precision%29) (TriggeredSeconds :type Float%20%28double-precision%29) (InputAction :type Input%20Action%20Object%20Reference :default "/Game/Blueprints/MainCharacter/Input/IA_SprintCC.IA_SprintCC"))
  ;[1 1 1] Movement
  (:Triggered
    (if ActionValue
      (Variables|Default|SetWalkMod 1.0)
      (else
        (Variables|Default|SetWalkMod (/ (Variables|Default|GetWalkSpeed) (Variables|Default|GetSprintSpeed)))))))

(event Input|EnhancedActionEvents|EnhancedInputActionIA_SlowTimeCC
  (params (ActionValue :type Boolean) (ElapsedSeconds :type Float%20%28double-precision%29) (TriggeredSeconds :type Float%20%28double-precision%29) (InputAction :type Input%20Action%20Object%20Reference :default "/Game/Blueprints/MainCharacter/Input/IA_SlowTimeCC.IA_SlowTimeCC"))
  (:Triggered
    (Utilities|FlowControl|FlipFlop
      (:A
        (Utilities|Time|SetGlobalTimeDilation (Variables|Default|GetSlowTimeAmount)))
      (:B
        (Utilities|Time|SetGlobalTimeDilation 1.0)))))

(event Input|EnhancedActionEvents|EnhancedInputActionIA_JumpCC
  (params (ActionValue :type Boolean) (ElapsedSeconds :type Float%20%28double-precision%29) (TriggeredSeconds :type Float%20%28double-precision%29) (InputAction :type Input%20Action%20Object%20Reference :default "/Game/Blueprints/MainCharacter/Input/IA_JumpCC.IA_JumpCC"))
  ;[1 1 1] Movement
  (:Triggered
    (bind _output_get (Variables|Default|SetJumpJustPressed ActionValue))
    (Variables|Default|SetJumpMaxHoldTime (Variables|Default|GetJump%20Max%20Hold%20Time))
    (if _output_get
      (if (<= (Variables|Default|GetCurrentSpeed) (Variables|Default|GetWalkSpeed))
        (Utilities|FlowControl|Delay (Variables|Default|GetJumpDelayTime))
        (Character|Jump)
        (else
          (Character|Jump)))
      (else
        (Character|StopJumping)))))

(event Input|EnhancedActionEvents|EnhancedInputActionIA_RagdollCC
  (params (ActionValue :type Boolean) (ElapsedSeconds :type Float%20%28double-precision%29) (TriggeredSeconds :type Float%20%28double-precision%29) (InputAction :type Input%20Action%20Object%20Reference :default "/Game/Blueprints/MainCharacter/Input/IA_RagdollCC.IA_RagdollCC"))
  (bind _returnvalue (Utilities|Name|MakeLiteralName "Hips"))
  (:Triggered
    (Class|PhysicalAnimationComponent|ApplyPhysicalAnimationProfileBelow (Variables|Default|GetPhysicalAnimation) _returnvalue "Loose" false false)
    (Class|SkeletalMeshComponent|SetAllBodiesBelowSimulatePhysics (Variables|Character|GetMesh) _returnvalue true true)
    (Variables|Default|SetIsRagdoll true)))

(event EventBeginPlay)

(event Collision|EventActorBeginOverlap
  (params (OtherActor :type Actor%20Object%20Reference)))

(event EventTick
  (params (DeltaSeconds :type Float%20%28single-precision%29))
  (bind _returnvalue (Pawn|GetMovementComponent))
  (bind _velocity (Variables|/Script/Engine.MovementComponent|GetVelocity _returnvalue))
  (bind (_x _y _z) (Math|Vector|BreakVector _velocity))
  (Variables|Default|SetVertSpeed _z)
  (Variables|Default|SetCurrentSpeed (Math|Vector|VectorLength (Math|Vector|MakeVector _x _y 0.0))))

(event EventPossessed
  (params (NewController :type Controller%20Object%20Reference))
  ;[1 1 1] Movement
  (bind _asplayer_controller (Utilities|Casting|CastToPlayerController NewController))
  (Input|EnableInput _asplayer_controller)
  (Input|AddMappingContext (PlayerController|LocalPlayerSubsystems|GetEnhancedInputLocalPlayerSubsystem _asplayer_controller) "/Game/Blueprints/MainCharacter/Input/IM_ThirdPersonCC.IM_ThirdPersonCC" 0 "(bIgnoreAllPressedKeysUntilRelease=True,bForceImmediately=False)"))

(fn ConstructionScript
  (Utilities|FlowControl|Sequence
    (:then_0
      (Variables|Default|SetmainCam (Variables|Default|GetCamera))
      (Variables|Default|SetskelMesh (Variables|Character|GetMesh)))
    (:then_1
      (Variables|/Script/Engine.CharacterMovementComponent|SetMaxWalkSpeed (Variables|Character|GetCharacterMovement) (Variables|Default|GetSprintSpeed))
      (Variables|Default|SetWalkMod (/ (Variables|Default|GetWalkSpeed) (Variables|Default|GetSprintSpeed)))
      (Class|PhysicalAnimationComponent|SetSkeletalMeshComponent (Variables|Default|GetPhysicalAnimation) (Variables|Character|GetMesh)))
    (:then_2
      (Variables|Default|SetJumpDelayTime 0.1))))